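; AC_NeptuneGates is an interactable component on Neptune level gates that opens a gate by destroying its owning actor.
; On interact, it compares its ItemID row name against the FactID at index 1 of the player's fact collection and destroys the gate on a match.
; Its LookAt function returns an empty prompt string.
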(event EventInteractwith
  (params (PlayerCharacter :type BP%20Jupiter%20Character%20Object%20Reference))
  (bind _ac_factcollectionsystem (Variables|/Game/Levels/Jupiter/BP_JupiterCharacter.BP_JupiterCharacter_C|GetAC_FactCollectionSystem PlayerCharacter))
  (Utilities|IsValid _ac_factcollectionsystem
    (:Is%20Valid
      (if (== (.rowname (Variables|Default|GetItemID)) (.factid (Utilities|Array|Get(acopy) (Variables|/Game/LogCollection/FactCollectData/AC_FactCollectionSystem.AC_FactCollectionSystem_C|GetFactCollection _ac_factcollectionsystem) 1)))
        (Actor|DestroyActor (Components|GetOwner))))))

(fn Lookat
  (return ""))