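; An ice patch trigger in the Uranus level that makes BP_CharacterKitty slide while inside it.
; Entering the box sets the character's ground friction to zero and lowers braking deceleration; leaving writes back fixed normal values rather than restoring saved ones.
; The construction script scales the box horizontally by a Size variable and toggles the static mesh's visibility with ShowPlane.
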(event OnComponentBeginOverlap(Box)
  (params (OverlappedComponent :type Primitive%20Component%20Object%20Reference) (OtherActor :type Actor%20Object%20Reference) (OtherComp :type Primitive%20Component%20Object%20Reference) (OtherBodyIndex :type Integer) (bFromSweep :type Boolean) (SweepResult :type Hit%20Result%20Structure%20%28by%20ref%29))
  (bind _asbp_character_kitty (Utilities|Casting|CastToBP_CharacterKitty OtherActor))
  (Variables|/Script/Engine.CharacterMovementComponent|SetGroundFriction (Variables|/Script/Engine.Character|GetCharacterMovement _asbp_character_kitty) 0.0)
  (Variables|/Script/Engine.CharacterMovementComponent|SetBrakingDecelerationWalking (Variables|/Script/Engine.Character|GetCharacterMovement _asbp_character_kitty) 3.5e+02))

(event OnComponentEndOverlap(Box)
  (params (OverlappedComponent :type Primitive%20Component%20Object%20Reference) (OtherActor :type Actor%20Object%20Reference) (OtherComp :type Primitive%20Component%20Object%20Reference) (OtherBodyIndex :type Integer))
  (bind _asbp_character_kitty (Utilities|Casting|CastToBP_CharacterKitty OtherActor))
  (Variables|/Script/Engine.CharacterMovementComponent|SetGroundFriction (Variables|/Script/Engine.Character|GetCharacterMovement _asbp_character_kitty) 8.0)
  (Variables|/Script/Engine.CharacterMovementComponent|SetBrakingDecelerationWalking (Variables|/Script/Engine.Character|GetCharacterMovement _asbp_character_kitty) 2e+03))

(event EventBeginPlay)

(event Collision|EventActorBeginOverlap
  (params (OtherActor :type Actor%20Object%20Reference)))

(event EventTick
  (params (DeltaSeconds :type Float%20%28single-precision%29)))

(fn ConstructionScript
  (bind _size (Variables|Default|GetSize))
  (Rendering|SetVisibility (Variables|Default|GetStaticMesh) (Variables|Default|GetShowPlane?) false)
  (Transformation|SetRelativeScale3D (Variables|Default|GetBox) (Math|Vector|MakeVector _size _size 1.0)))