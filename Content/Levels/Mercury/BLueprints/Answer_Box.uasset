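; Answer Box actor for a puzzle that opens a linked Door when the entered Input matches the Answer read from NumberGen.
; Overlapping the Box disables player input, shows the mouse cursor and opens the Answer widget; Exit reverses this.
; Four display meshes get dynamic material instances, and SetNewImg swaps the texture on a chosen one using ImageArray.
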(event OnComponentBeginOverlap(Box)
  (params (OverlappedComponent :type Primitive%20Component%20Object%20Reference) (OtherActor :type Actor%20Object%20Reference) (OtherComp :type Primitive%20Component%20Object%20Reference) (OtherBodyIndex :type Integer) (bFromSweep :type Boolean) (SweepResult :type Hit%20Result%20Structure%20%28by%20ref%29))
  (Variables|Default|SetPlayer OtherActor)
  (Variables|/Script/Engine.PlayerController|SetbShowMouseCursor (Game|GetPlayerController 0) true)
  (Input|DisableInput (Variables|Default|GetPlayer) 0)
  (bind _returnvalue (UserInterface|CreateWidget "/Game/Levels/Mercury/BLueprints/Answer.Answer_C"))
  (UserInterface|Viewport|AddtoViewport _returnvalue 0))

(event Custom|SendAnswer
  (if (== (stale EventBeginPlay _output_get) (Variables|Default|GetInput))
    (Variables|/Game/Levels/Mercury/BLueprints/Door.Door_C|SetIsOpen (Variables|Default|GetDoor) (== (stale EventBeginPlay _output_get) (Variables|Default|GetInput)))))

(event Custom|Exit
  (Variables|/Script/Engine.PlayerController|SetbShowMouseCursor (Game|GetPlayerController 0) false)
  (Input|EnableInput (Variables|Default|GetPlayer) 0)
  (bind _foundwidgets (Widget|GetAllWidgetsOfClass "/Game/Levels/Mercury/BLueprints/Answer.Answer_C" true))
  (for _array_element _foundwidgets
    (Widget|RemovefromParent _array_element)))

(event Custom|SetNewImg
  (params (BoxNumb :type Integer) (Value :type Integer))
  (bind _boxmesharray (Variables|Default|GetBoxMeshArray))
  (bind _output (Utilities|Array|Get(acopy) _boxmesharray BoxNumb))
  (bind _returnvalue (Rendering|Material|CreateDynamicMaterialInstance _output 1 (Rendering|Material|GetMaterial _output 1) (Utilities|String|StringToName (Utilities|String|Append (Utilities|String|MakeLiteralString "Display_Material") (Utilities|GetObjectName (stale EventBeginPlay _array_element)))) :!class /Script/Engine.PrimitiveComponent))
  (Rendering|Material|SetMaterial _output 1 _returnvalue)
  (Rendering|Material|SetTextureParameterValue _returnvalue "Texture" (Utilities|Array|Get(acopy) (Variables|Default|GetImageArray) Value)))

(event EventBeginPlay
  (Utilities|FlowControl|Sequence
    (:then_0
      (Variables|Default|SetBoxMeshArray (Utilities|Array|MakeArray (Variables|Default|GetAnswerBox_Answer1) (Variables|Default|GetAnswerBox_Answer2) (Variables|Default|GetAnswerBox_Answer3) (Variables|Default|GetAnswerBox_Answer4))))
    (:then_1
      (bind _output_get (Variables|Default|SetAnswer (Variables|/Game/Levels/Mercury/BLueprints/NumberGen.NumberGen_C|GetAnswer (Variables|Default|GetNumberGen)))))
    (:then_2
      (for _array_element (Variables|Default|GetBoxMeshArray)
        (bind _returnvalue (Rendering|Material|CreateDynamicMaterialInstance _array_element 1 "/Game/Levels/Mercury/Meshs/Materials/Display_Master.Display_Master" (Utilities|String|StringToName (Utilities|String|Append (Utilities|String|MakeLiteralString "Display_Material") (Utilities|GetObjectName _array_element))) :!class /Script/Engine.PrimitiveComponent)) ; Makes a Material Instance for each  mesh
        (Rendering|Material|SetMaterial _array_element 1 _returnvalue) ; Apply that bad boi
      ))))

(fn ConstructionScript)