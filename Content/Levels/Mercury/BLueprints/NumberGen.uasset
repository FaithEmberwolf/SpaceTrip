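; Number puzzle actor in the Mercury level that picks two random four-digit numbers on BeginPlay, stores their sum as Answer and displays both numbers.
; Each number is split into digit characters, matched by index to a top or bottom row of four meshes.
; Every mesh gets a dynamic material instance on slot 1, with its Texture parameter set to that digit's image from ImageArray.
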(event EventBeginPlay
  (Utilities|FlowControl|Sequence
    (:then_0
      ;[1 1 1] NumberGen
      (bind _output_get (Variables|Default|SetNumber1 (Math|Random|RandomIntegerinRange 1000 4999)))
      (bind _output_get_2 (Variables|Default|SetNumber2 (Math|Random|RandomIntegerinRange 1000 4999)))
      (Variables|Default|SetAnswer (+ _output_get _output_get_2)))
    (:then_1
      ;[1 1 1] GenerateNumb into String Array & MeshArrays
      (Variables|Default|SetTopArray (Utilities|String|GetCharacterArrayfromString (Utilities|String|ToString(Integer) (Variables|Default|GetNumber1))))
      (Variables|Default|SetBottomArray (Utilities|String|GetCharacterArrayfromString (Utilities|String|ToString(Integer) (Variables|Default|GetNumber2))))
      (Variables|Default|SetTopArrayMesh (Utilities|Array|MakeArray (Variables|Default|GetTop1) (Variables|Default|GetTop2) (Variables|Default|GetTop3) (Variables|Default|GetTop4)))
      (Variables|Default|SetBottomArrayMesh (Utilities|Array|MakeArray (Variables|Default|GetBottom1) (Variables|Default|GetBottom2) (Variables|Default|GetBottom3) (Variables|Default|GetBottom4))))
    (:then_2
      ;[1 1 1] Generate Marials for Top Row
      (for (_array_element _array_index) (Variables|Default|GetTopArrayMesh)
        (bind _returnvalue (Rendering|Material|CreateDynamicMaterialInstance _array_element 1 0 (Utilities|String|StringToName (Utilities|String|Append (Utilities|String|MakeLiteralString "Display_Material") (Utilities|GetObjectName _array_element))) :!class /Script/Engine.PrimitiveComponent)) ; Makes a Material Instance for each  mesh
        (Rendering|Material|SetTextureParameterValue _returnvalue "Texture" (Utilities|Array|Get(acopy) (Variables|Default|GetImageArray) (Math|Conversions|ToInteger(Byte) (Utilities|Array|Get(acopy) (Variables|Default|GetTopArray) _array_index)))) ; Sets the image to be that Image via the string array
        (Rendering|Material|SetMaterial _array_element 1 _returnvalue) ; Apply that bad boi
      )
      ;[1 1 1] Generate Materials for Bottom Row :3
      (for (_array_element_2 _array_index_2) (Variables|Default|GetBottomArrayMesh)
        (bind _returnvalue_2 (Rendering|Material|CreateDynamicMaterialInstance _array_element_2 1 0 (Utilities|String|StringToName (Utilities|String|Append (Utilities|String|MakeLiteralString "Display_Material") (Utilities|GetObjectName _array_element_2))) :!class /Script/Engine.PrimitiveComponent))
        (Rendering|Material|SetTextureParameterValue _returnvalue_2 "Texture" (Utilities|Array|Get(acopy) (Variables|Default|GetImageArray) (Math|Conversions|ToInteger(Byte) (Utilities|Array|Get(acopy) (Variables|Default|GetBottomArray) _array_index_2))))
        (Rendering|Material|SetMaterial _array_element_2 1 _returnvalue_2)))))

(fn ConstructionScript)