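; Actor component for the player character that handles collecting planet facts and interacting with fact objects and Neptune gates.
; Each tick a forward sphere trace from the player sets LookAtActor and prints its look-at message.
; The interaction input messages that actor's AC_FactData and AC_NeptuneGates components, passing the owning BP_JupiterCharacter.
; CollectFact stores FactCollected and copies that entry of FactCollection into fixed index 1, leaving FactId unused.
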(event Input|EnhancedActionEvents|EnhancedInputActionIA_ObjectInteraction
  (params (ActionValue :type Vector%202D%20Structure) (ElapsedSeconds :type Float%20%28double-precision%29) (TriggeredSeconds :type Float%20%28double-precision%29) (InputAction :type Input%20Action%20Object%20Reference :default "/Game/ThirdPerson/Input/Actions/IA_ObjectInteraction.IA_ObjectInteraction"))
  (bind _lookatactor (Variables|Default|GetLookAtActor))
  ;[1 1 1] Interact with Gates
  (:Started
    (Utilities|IsValid _lookatactor
      (:Is%20Valid
        (Class|IInteractionInterface|Interactwith(Message) (Actor|GetComponentbyClass _lookatactor "/Game/Levels/Neptune/Assets/Doors/AC_NeptuneGates.AC_NeptuneGates_C") (.AsBP%20Jupiter%20Character (Utilities|Casting|CastToBP_JupiterCharacter (Components|GetOwner))))))))

(event Input|EnhancedActionEvents|EnhancedInputActionIA_ObjectInteraction
  (params (ActionValue :type Vector%202D%20Structure) (ElapsedSeconds :type Float%20%28double-precision%29) (TriggeredSeconds :type Float%20%28double-precision%29) (InputAction :type Input%20Action%20Object%20Reference :default "/Game/ThirdPerson/Input/Actions/IA_ObjectInteraction.IA_ObjectInteraction"))
  (bind _lookatactor (Variables|Default|GetLookAtActor))
  ;[1 1 1] Pick up Object
  (:Started
    (Utilities|IsValid _lookatactor
      (:Is%20Valid
        (Class|IInteractionInterface|Interactwith(Message) (Actor|GetComponentbyClass _lookatactor "/Game/LogCollection/FactCollectData/AC_FactData.AC_FactData_C") (.AsBP%20Jupiter%20Character (Utilities|Casting|CastToBP_JupiterCharacter (Components|GetOwner))))))))

(event EventBeginPlay
  (Utilities|Array|Resize (Variables|Default|GetFactCollection) (Math|Conversions|ToInteger(Boolean) (Variables|Default|GetFact%20Collected))))

(event EventTick
  (params (DeltaSeconds :type Float%20%28single-precision%29))
  (CallFunction|InteractionTracing))

(fn CollectFact
  (params (FactId :type Name) (Collected? :type Boolean))
  (bind _output_get (Variables|Default|SetFact%20Collected Collected?))
  (CallFunction|AddtoPlanetRegistry FactId _output_get)
  (if true
    _))

(fn AddtoPlanetRegistry
  (params (FactID :type Name) (FactNumber :type Integer))
  (bind _factcollection (Variables|Default|GetFactCollection))
  (bind _output (Utilities|Array|Get(acopy) _factcollection FactNumber))
  (Utilities|Array|SetArrayElem _factcollection 1 (Utilities|Struct|MakeF_FactStruct (.factid _output) (.description _output) (.hasbeencollected _output) (.factnumber _output))))

(fn InteractionTracing
  (bind _returnvalue (Game|GetPlayerCharacter 0))
  (bind _returnvalue_2 (Transformation|GetActorLocation _returnvalue))
  (bind (_outhit _returnvalue_3) (Collision|SphereTraceByChannel _returnvalue_2 (+ _returnvalue_2 (* (Transformation|GetActorForwardVector _returnvalue) (Variables|Default|GetInteractionRange))) 6e+01 "TraceTypeQuery3" false (Utilities|Array|MakeArray (Components|GetOwner)) "None"))
  (if _returnvalue_3
    (if (!= (.HitActor (Collision|BreakHitResult _outhit)) (Variables|Default|GetLookAtActor))
      (bind _output_get (Variables|Default|SetLookAtActor (.HitActor (Collision|BreakHitResult _outhit))))
      (bind _message (Class|IInteractionInterface|Lookat(Message) _output_get))
      (Development|PrintString (Utilities|String|ToString(Text) _message)))
    (else
      (Variables|Default|SetLookAtActor 0))))