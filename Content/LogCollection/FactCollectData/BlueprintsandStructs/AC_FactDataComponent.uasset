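; Actor component that turns its owner into a collectible fact pickup for the player's fact log.
; On BeginPlay it enables replication on the owning actor.
; Interactwith passes the FactID row name to the player's ACFactCollectionSystem via AddToLog, then marks itself collected and destroys the owner without checking whether the add succeeded.
; LookAt returns an empty string, so it supplies no look-at text.
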(event EventBeginPlay
  (Networking|SetReplicates (Components|GetOwner) true))

(event EventInteractwith
  (params (PlayerCharacter :type BP%20Jupiter%20Character%20Object%20Reference))
  (bind _ac_factcollectionsystem (Variables|/Game/Levels/Jupiter/BP_JupiterCharacter.BP_JupiterCharacter_C|GetAC_FactCollectionSystem PlayerCharacter))
  (Utilities|IsValid _ac_factcollectionsystem
    (:Is%20Valid
      (Default|AddtoLog _ac_factcollectionsystem (.rowname (Variables|Default|GetFactID)) 1)
      (if true
        (Variables|Default|SetHasBeenCollected true)
        (Actor|DestroyActor (Components|GetOwner))))))

(fn Lookat
  (return ""))