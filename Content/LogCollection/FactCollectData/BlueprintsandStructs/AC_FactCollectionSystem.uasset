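; Actor component for fact collection that detects what the player character is facing, with fact logging stubbed out.
; Every tick it sphere-traces forward from player 0's location out to InteractionRange, ignoring its owner.
; A newly hit actor is cached as LookAtActor and its LookAtMessage result is printed; a miss clears the cache.
; AddToLog, marked as the way of storing facts, is still empty.
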(event EventTick
  (params (DeltaSeconds :type Float%20%28single-precision%29))
  (CallFunction|InteractionTracing))

(fn AddtoLog
  ;[1 1 1] Way of Storing Facts
)

(fn InteractionTracing
  (bind _returnvalue (Game|GetPlayerCharacter 0))
  (bind _returnvalue_2 (Transformation|GetActorLocation _returnvalue))
  ;[1 1 1] Tracing Section
  (bind (_outhit _returnvalue_3) (Collision|SphereTraceByChannel _returnvalue_2 (+ _returnvalue_2 (* (Transformation|GetActorForwardVector _returnvalue) (Variables|Default|GetInteractionRange))) 15.0 "TraceTypeQuery3" false (Utilities|Array|MakeArray (Components|GetOwner)) "None"))
  (if _returnvalue_3
    (if (!= (.HitActor (Collision|BreakHitResult _outhit)) (Variables|Default|GetLookAtActor))
      (bind _output_get (Variables|Default|SetLookAtActor (.HitActor (Collision|BreakHitResult _outhit))))
      (bind _message (Class|IInteractionInterface|Lookat(Message) _output_get))
      (Development|PrintString (Utilities|String|ToString(Text) _message)))
    (else
      (Variables|Default|SetLookAtActor 0))))