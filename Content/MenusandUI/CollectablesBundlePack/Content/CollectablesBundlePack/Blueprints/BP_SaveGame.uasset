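; BP_SaveGame is a save-game data container for the collectables pack, storing player progression and collection state.
; It holds XP, level and top bar progress, six collectable sets with their counts, and a record of destroyed actors.
; A single setter writes every field at once and a matching getter returns them all, with no other logic.
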(fn GetSaveGameValues
  (return (Variables|Default|GetXP) (Variables|Default|GetMax%20XP) (Variables|Default|GetOld%20XP) (Variables|Default|GetTop%20Bar%20Percentage) (Variables|Default|GetLevel) (Variables|Default|GetCollectables%2001) (Variables|Default|GetCollectables%2002) (Variables|Default|GetCollectables%2003) (Variables|Default|GetCollectables%2004) (Variables|Default|GetCollectables%2005) (Variables|Default|GetCollectables%2006) (Variables|Default|GetNumber%20of%20Collectables%2001) (Variables|Default|GetNumber%20of%20Collectables%2002) (Variables|Default|GetNumber%20of%20Collectables%2003) (Variables|Default|GetNumber%20of%20Collectables%2004) (Variables|Default|GetNumber%20of%20Collectables%2005) (Variables|Default|GetNumber%20of%20Collectables%2006) (Variables|Default|GetDestroyed%20Actors)))

(fn SetSaveGameValues
  (params (XP :type Float%20%28single-precision%29) (Max%20XP :type Float%20%28single-precision%29) (Old%20XP :type Float%20%28single-precision%29) (Top%20Bar%20Percentage :type Float%20%28single-precision%29) (Level :type Integer) (Collectables%2001 :type Integer) (Collectables%2002 :type Integer) (Collectables%2003 :type Integer) (Collectables%2004 :type Integer) (Collectables%2005 :type Integer) (Collectables%2006 :type Integer) (Number%20of%20Collectables%2001 :type Integer) (Number%20of%20Collectables%2002 :type Integer) (Number%20of%20Collectables%2003 :type Integer) (Number%20of%20Collectables%2004 :type Integer) (Number%20of%20Collectables%2005 :type Integer) (Number%20of%20Collectables%2006 :type Integer) (Destroyed%20Actors :type Array%20of%20Names))
  (Variables|Default|SetXP XP)
  (Variables|Default|SetMax%20XP Max%20XP)
  (Variables|Default|SetOld%20XP Old%20XP)
  (Variables|Default|SetTop%20Bar%20Percentage Top%20Bar%20Percentage)
  (Variables|Default|SetLevel Level)
  (Variables|Default|SetCollectables%2001 Collectables%2001)
  (Variables|Default|SetCollectables%2002 Collectables%2002)
  (Variables|Default|SetCollectables%2003 Collectables%2003)
  (Variables|Default|SetCollectables%2004 Collectables%2004)
  (Variables|Default|SetCollectables%2005 Collectables%2005)
  (Variables|Default|SetCollectables%2006 Collectables%2006)
  (Variables|Default|SetNumber%20of%20Collectables%2001 Number%20of%20Collectables%2001)
  (Variables|Default|SetNumber%20of%20Collectables%2002 Number%20of%20Collectables%2002)
  (Variables|Default|SetNumber%20of%20Collectables%2003 Number%20of%20Collectables%2003)
  (Variables|Default|SetNumber%20of%20Collectables%2004 Number%20of%20Collectables%2004)
  (Variables|Default|SetNumber%20of%20Collectables%2005 Number%20of%20Collectables%2005)
  (Variables|Default|SetNumber%20of%20Collectables%2006 Number%20of%20Collectables%2006)
  (Variables|Default|SetDestroyed%20Actors Destroyed%20Actors))