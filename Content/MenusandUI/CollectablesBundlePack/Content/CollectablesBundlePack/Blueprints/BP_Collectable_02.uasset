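; BP_Collectable_02 is a collectable pickup that the player collects by overlapping its sphere.
; On BeginPlay it writes the count of its class to the GameInstance and destroys itself if its ItemToFind is already recorded as destroyed.
; Collecting increments the GameInstance tally, shows progress on the HUD and awards XP, with more for completing the set.
; It then registers ItemToFind with the GameInstance and destroys itself.
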(event OnComponentBeginOverlap(Sphere)
  (params (OverlappedComponent :type Primitive%20Component%20Object%20Reference) (OtherActor :type Actor%20Object%20Reference) (OtherComp :type Primitive%20Component%20Object%20Reference) (OtherBodyIndex :type Integer) (bFromSweep :type Boolean) (SweepResult :type Hit%20Result%20Structure%20%28by%20ref%29))
  (if (== OtherActor (CallFunction|GetPlayerCharacter))
    (CallFunction|Collect)))

(event EventBeginPlay
  (bind _return_value (CallFunction|GetGameInstance))
  (bind _outactors (Actor|GetAllActorsOfClass "BP_Collectable_02_C"))
  (Variables|/Game/CollectablesBundlePack/Blueprints/BP_GameInstance.BP_GameInstance_C|SetNumber%20of%20Collectables%2002 _return_value (Utilities|Array|Length _outactors))
  (bind _destroyed (Default|CheckifDestroyed? _return_value (Variables|Default|GetItem%20to%20Find)))
  (if _destroyed
    (Actor|DestroyActor)))

(fn ConstructionScript)

(fn Collect
  (bind _return_value (CallFunction|GetGameInstance))
  (bind _return_value_2 (CallFunction|GetPlayerHUD))
  (bind _number_of_collectables_02 (Variables|/Game/CollectablesBundlePack/Blueprints/BP_GameInstance.BP_GameInstance_C|GetNumber%20of%20Collectables%2002 _return_value))
  (bind _w_collectiblefound (Variables|/Game/CollectablesBundlePack/Blueprints/BP_HUD.BP_HUD_C|GetW_CollectibleFound _return_value_2))
  (Variables|/Game/CollectablesBundlePack/Blueprints/BP_GameInstance.BP_GameInstance_C|SetCollectables%2002 _return_value (+ (Variables|/Game/CollectablesBundlePack/Blueprints/BP_GameInstance.BP_GameInstance_C|GetCollectables%2002 _return_value) 1))
  (Variables|/Game/CollectablesBundlePack/Widgets/W_CollectableFound.W_CollectableFound_C|SetNumber%20of%20Collectables _w_collectiblefound _number_of_collectables_02)
  (Variables|/Game/CollectablesBundlePack/Widgets/W_CollectableFound.W_CollectableFound_C|SetCollectables _w_collectiblefound (Variables|/Game/CollectablesBundlePack/Blueprints/BP_GameInstance.BP_GameInstance_C|GetCollectables%2002 _return_value))
  (Variables|/Game/CollectablesBundlePack/Widgets/W_CollectableFound.W_CollectableFound_C|SetCollectable%20Name _w_collectiblefound (Variables|Default|GetCollectable%20Name))
  (Default|DisplayCollectableFound _return_value_2)
  (if (not (== (Variables|/Game/CollectablesBundlePack/Blueprints/BP_GameInstance.BP_GameInstance_C|GetCollectables%2002 _return_value) _number_of_collectables_02))
    (Default|AddXP _return_value_2 0.1)
    (else
      (Default|AddXP _return_value_2 1.7)))
  (Default|DestroyActor _return_value (Variables|Default|GetItem%20to%20Find))
  (Actor|DestroyActor))