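; Actor component for a fact collection system, apparently recording facts the player collects, though the logic is unfinished.
; CollectFact only sets a single FactCollected flag, ignoring its FactId, and holds disconnected inventory stacking code that never runs.
; AddToPlanetRegistry, despite its name, adds nothing: it searches FactCollection for a matching, already collected FactID and returns whether it was found, with its index.
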(event EventBeginPlay)

(event EventTick
  (params (DeltaSeconds :type Float%20%28single-precision%29)))

(fn CollectFact
  (params (FactId :type Name) (Collected? :type Boolean))
  (Variables|Default|SetFact%20Collected Collected?))

(fn AddtoPlanetRegistry
  (params (FactID :type Name))
  (for (_array_element _array_index) (Variables|Default|GetFactCollection)
    (if (== (.FactID (Utilities|Struct|BreakF_FactStruct _array_element)) FactID)
      (if (.HasBeenCollected (Utilities|Struct|BreakF_FactStruct _array_element))
        (return true _array_index))))
  (return false -1))