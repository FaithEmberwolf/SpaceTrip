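; BP_Spaceship_Character is the player-controlled spaceship Character, handling movement input and opening the pause menu.
; Move Forward and Move Right axes add movement along the capsule's forward and right vectors, and the Jump action triggers the standard Character jump.
; P or Escape creates WBP_PauseMenu, shows the mouse cursor and switches to UI-only input, without pausing the game in this graph.
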(event EventBeginPlay)

(event Collision|EventActorBeginOverlap
  (params (OtherActor :type Actor%20Object%20Reference)))

(event EventTick
  (params (DeltaSeconds :type Float%20%28single-precision%29)))

(event Input|ActionEvents|InputActionJump
  (params (Key :type Key%20Structure))
  (:Pressed
    (Character|Jump)))

(event Input|AxisEvents|InputAxisMoveForward
  (params (AxisValue :type Float%20%28single-precision%29))
  ;[1 1 1] Movement
  (Pawn|Input|AddMovementInput (Math|Vector|GetForwardVector (Variables|Collision|GetCapsuleComponent)) AxisValue false))

(event Input|AxisEvents|InputAxisMoveRight
  (params (AxisValue :type Float%20%28single-precision%29))
  ;[1 1 1] Movement
  (Pawn|Input|AddMovementInput (Math|Vector|GetRightVector (Variables|Collision|GetCapsuleComponent)) AxisValue false))

(event Input|KeyboardEvents|P
  (params (Key :type Key%20Structure))
  (bind _returnvalue (Game|GetPlayerController 0))
  ;[1 1 1] Pause Menu
  (:Pressed
    (bind _returnvalue_2 (UserInterface|CreateWidget "/Game/MenusandUI/Menus/PauseMenu/WBP_PauseMenu.WBP_PauseMenu_C"))
    (UserInterface|Viewport|AddtoViewport _returnvalue_2 0)
    (Variables|/Script/Engine.PlayerController|SetbShowMouseCursor _returnvalue true)
    (Input|SetInputModeUIOnly _returnvalue 0 "DoNotLock" false)))

(event Input|KeyboardEvents|Escape
  (params (Key :type Key%20Structure))
  (bind _returnvalue (Game|GetPlayerController 0))
  ;[1 1 1] Pause Menu
  (:Pressed
    (bind _returnvalue_2 (UserInterface|CreateWidget "/Game/MenusandUI/Menus/PauseMenu/WBP_PauseMenu.WBP_PauseMenu_C"))
    (UserInterface|Viewport|AddtoViewport _returnvalue_2 0)
    (Variables|/Script/Engine.PlayerController|SetbShowMouseCursor _returnvalue true)
    (Input|SetInputModeUIOnly _returnvalue 0 "DoNotLock" false)))

(fn ConstructionScript)