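; Save game object that stores the player's planetary collectable progress.
; It holds a collectables value and a count for the Sun and each planet through Pluto, plus a DestroyedActors record.
; SetSaveGameValues writes every field in one call, and GetSaveGameValues returns them all together.
; It contains no disk save or load logic, only the data and these two bulk accessors.
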(fn SetSaveGameValues
  (params (Sun%20Collectables :type Integer) (Mercury%20Collectables :type Integer) (Venus%20Collectables :type Integer) (Earth%20Collectables :type Integer) (Mars%20Collectables :type Integer) (Jupiter%20Collectables :type Integer) (Saturn%20Collectables :type Integer) (Uranus%20Collectables :type Integer) (Neptune%20Collectables :type Integer) (Pluto%20Collectables :type Integer) (Number%20of%20Sun :type Integer) (Number%20of%20Mercury :type Integer) (Number%20of%20Venus :type Integer) (Number%20of%20Earth :type Integer) (Number%20of%20Mars :type Integer) (Number%20of%20Jupiter :type Integer) (Number%20of%20Saturn :type Integer) (Number%20of%20Uranus :type Integer) (Number%20of%20Neptune :type Integer) (Number%20of%20Pluto :type Integer) (Destroyed%20Actors :type Array%20of%20Names))
  (Variables|Default|SetSun%20Collectables Sun%20Collectables)
  (Variables|Default|SetMercury%20Collectables Mercury%20Collectables)
  (Variables|Default|SetVenus%20Collectables Venus%20Collectables)
  (Variables|Default|SetEarth%20Collectables Earth%20Collectables)
  (Variables|Default|SetMars%20Collectables Mars%20Collectables)
  (Variables|Default|SetJupiter%20Collectables Jupiter%20Collectables)
  (Variables|Default|SetSaturn%20Collectables Saturn%20Collectables)
  (Variables|Default|SetUranus%20Collectables Uranus%20Collectables)
  (Variables|Default|SetNeptune%20Collectables Neptune%20Collectables)
  (Variables|Default|SetPluto%20Collectables Pluto%20Collectables)
  (Variables|Default|SetNumber%20Of%20Sun Number%20of%20Sun)
  (Variables|Default|SetNumber%20Of%20Mercury Number%20of%20Mercury)
  (Variables|Default|SetNumber%20Of%20Venus Number%20of%20Venus)
  (Variables|Default|SetNumber%20Of%20Earth Number%20of%20Earth)
  (Variables|Default|SetNumber%20Of%20Mars Number%20of%20Mars)
  (Variables|Default|SetNumber%20Of%20Jupiter Number%20of%20Jupiter)
  (Variables|Default|SetNumber%20Of%20Saturn Number%20of%20Saturn)
  (Variables|Default|SetNumber%20Of%20Uranus Number%20of%20Uranus)
  (Variables|Default|SetNumber%20Of%20Neptune Number%20of%20Neptune)
  (Variables|Default|SetNumber%20Of%20Pluto Number%20of%20Pluto)
  (Variables|Default|SetDestroyed%20Actors Destroyed%20Actors))

(fn GetSaveGameValues
  (return (Variables|Default|GetSun%20Collectables) (Variables|Default|GetMercury%20Collectables) (Variables|Default|GetVenus%20Collectables) (Variables|Default|GetEarth%20Collectables) (Variables|Default|GetMars%20Collectables) (Variables|Default|GetJupiter%20Collectables) (Variables|Default|GetSaturn%20Collectables) (Variables|Default|GetUranus%20Collectables) (Variables|Default|GetNeptune%20Collectables) (Variables|Default|GetPluto%20Collectables) (Variables|Default|GetNumber%20Of%20Sun) (Variables|Default|GetNumber%20Of%20Mercury) (Variables|Default|GetNumber%20Of%20Venus) (Variables|Default|GetNumber%20Of%20Earth) (Variables|Default|GetNumber%20Of%20Mars) (Variables|Default|GetNumber%20Of%20Jupiter) (Variables|Default|GetNumber%20Of%20Saturn) (Variables|Default|GetNumber%20Of%20Uranus) (Variables|Default|GetNumber%20Of%20Neptune) (Variables|Default|GetNumber%20Of%20Pluto) (Variables|Default|GetDestroyed%20Actors)))