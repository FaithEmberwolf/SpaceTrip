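; BP_SunCollectables is the sun collectable item, tracked through a running count in the game instance.
; Collect increments SunCollectables there, then fills NumberOfCollectables from NumberOfSun alongside the item's name and description.
; The event graph and construction script are empty, and leftover nodes for a count comparison, log menu and HUD are unconnected.
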(event EventBeginPlay)

(event Collision|EventActorBeginOverlap
  (params (OtherActor :type Actor%20Object%20Reference)))

(event EventTick
  (params (DeltaSeconds :type Float%20%28single-precision%29)))

(fn ConstructionScript)

(fn Collect
  (bind _asbp_game_instance (CallFunction|GetGameInstance))
  (Variables|/Game/collectables/Blueprints/BP_GameInstance.BP_GameInstance_C|SetSun%20Collectables _asbp_game_instance (+ (Variables|/Game/collectables/Blueprints/BP_GameInstance.BP_GameInstance_C|GetSun%20Collectables _asbp_game_instance) 1))
  (Variables|Default|SetNumber%20of%20Collectables (Variables|/Game/collectables/Blueprints/BP_GameInstance.BP_GameInstance_C|GetNumber%20Of%20Sun _asbp_game_instance))
  (Variables|Default|SetCollectable%20Name (Variables|Default|GetCollectable%20Name))
  (Variables|Default|SetCollectable%20Description (Variables|Default|GetCollectable%20Description)))